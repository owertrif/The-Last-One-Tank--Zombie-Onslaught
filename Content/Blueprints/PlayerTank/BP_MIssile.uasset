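; BP_MIssile is a missile projectile, filed under PlayerTank, that adds an animated explosion to its parent class's explode behavior.
; On OnExplode it disables collision, zeroes its speed, clears its sprite and plays the Explode flipbook once at enlarged scale.
; The parent's OnExplode is deferred until the flipbook finishes, through a bound finished-playing event.
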(event Custom|FinishExploding
  (|CallParentFunction))

(event EventBeginPlay)

(event Collision|EventActorBeginOverlap
  (params (OtherActor :type Actor%20Object%20Reference)))

(event EventTick
  (params (DeltaSeconds :type Float%20%28single-precision%29)))

(event EventOnExplode
  (bind _paperflipbook (Variables|Default|GetPaperFlipbook))
  (Collision|SetActorEnableCollision false)
  (Sprite|SetFlipbook _paperflipbook "/Game/assets/tank/textures/Explode.Explode")
  (Transformation|SetWorldScale3D _paperflipbook "2.000000,2.000000,2.000000")
  (Audio|Components|Audio|Play _paperflipbook)
  (Components|Timeline|SetLooping _paperflipbook false)
  (EventDispatchers|BindEventtoOnFinishedPlaying _paperflipbook (delegate Custom|FinishExploding))
  (Rendering|Components|Sprite|SetSprite (Variables|Default|GetPaperSprite) 0)
  (Variables|Default|SetSpeed 0.0))

(fn ConstructionScript)