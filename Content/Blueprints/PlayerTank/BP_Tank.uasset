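; Player tank Blueprint that handles the UI side of death and leveling up.
; TankDie waits briefly before showing the death screen, while LevelUp shows its widget immediately.
; Both events then pause the game, switch input to UI only and hide the virtual joystick.
; Nothing in this file triggers these events or restores gameplay afterward.
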(event EventBeginPlay)

(event Collision|EventActorBeginOverlap
  (params (OtherActor :type Actor%20Object%20Reference)))

(event EventTick
  (params (DeltaSeconds :type Float%20%28single-precision%29)))

(event EventTankDie
  (params (DamageType :type EDamageType%20Enum :default "Unknown"))
  (bind _returnvalue (Game|GetPlayerController 0))
  (Utilities|FlowControl|Delay 2.0)
  (bind _returnvalue_2 (UserInterface|CreateWidget "/Game/Blueprints/UI/DeathScreen_WBP.DeathScreen_WBP_C"))
  (UserInterface|Viewport|AddtoViewport _returnvalue_2 0)
  (Game|SetGamePaused true)
  (Input|SetInputModeUIOnly _returnvalue 0 "DoNotLock" false)
  (Class|PlayerController|SetVirtualJoystickVisibility _returnvalue false))

(event EventLevelUp
  (bind _returnvalue (Game|GetPlayerController 0))
  (bind _returnvalue_2 (UserInterface|CreateWidget "/Game/Blueprints/UI/LevelUp_WBP.LevelUp_WBP_C"))
  (UserInterface|Viewport|AddtoViewport _returnvalue_2 0)
  (Game|SetGamePaused true)
  (Input|SetInputModeUIOnly _returnvalue 0 "DoNotLock" false)
  (Class|PlayerController|SetVirtualJoystickVisibility _returnvalue false))

(fn ConstructionScript)