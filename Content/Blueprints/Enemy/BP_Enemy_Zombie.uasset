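; BP_Enemy_Zombie is a zombie enemy Blueprint that supplies Paper2D flipbook animations for the walk, attack and death events.
; Walk and attack loop their flipbooks, scaling play rate from the distance walked and the attack cooldown respectively.
; Death disables collision, plays the die flipbook from the start and runs a timeline that destroys the actor when it finishes.
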(event EventBeginPlay)

(event Collision|EventActorBeginOverlap
  (params (OtherActor :type Actor%20Object%20Reference)))

(event EventTick
  (params (DeltaSeconds :type Float%20%28single-precision%29)))

(event EventEnemyDie
  (params (DamageType :type EDamageType%20Enum :default "Unknown"))
  (Collision|SetActorEnableCollision false)
  (Class|TankStatics|PlayFlipbook (Variables|Default|GetPaperFlipbook) "/Game/assets/zomie/Zombie_Die.Zombie_Die" false 1.0 true)
  (Utilities|FlowControl|Sequence
    (:then_0
      (Timeline|Timeline PlayFromStart
        (:Finished
          (Actor|DestroyActor))))))

(event EventEnemyWalk
  (params (DeltaSeconds :type Float%20%28single-precision%29) (DistanceWalked :type Float%20%28single-precision%29))
  (Class|TankStatics|PlayFlipbook (Variables|Default|GetPaperFlipbook) "/Game/assets/zomie/ZombieWalk.ZombieWalk" true (/ DistanceWalked 5.0) false))

(event EventEnemyAttack
  (params (DeltaSeconds :type Float%20%28single-precision%29) (AtkCooldown :type Float%20%28single-precision%29))
  (Class|TankStatics|PlayFlipbook (Variables|Default|GetPaperFlipbook) "/Game/assets/zomie/ZombieAttack.ZombieAttack" true (/ AtkCooldown 2.7) false))

(fn ConstructionScript)